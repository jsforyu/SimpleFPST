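; Base enemy character that runs an AI behavior tree, fights the first-person player and shows a health bar widget.
; Pawn sensing, or taking damage, writes the player to the AttackTarget blackboard key.
; Random attack montages use a notify to sphere-trace forward and damage the player, then fire an end dispatcher for listeners.
; Non-lethal hits play a reaction that halts movement; death stops AI, disables collision and notifies the GameMode.
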(event `self.ReceiveBeginPlay`
  (bind _output_get (set `self.AIController` (`AIBlueprintHelperLibrary.GetAIController` self)))
  (`AIController.RunBehaviorTree` _output_get "/Game/Charactors/Enemys/BluePoint/BT/BT_Enemy.BT_Enemy")
  (set `self.MaxHealth` (`self.Health`))
  ;[1 1 1] 设置敌人血条
  (bind _returnvalue (`|CreateWidget` "/Game/FirstPerson/Blueprints/UI/UMG_EnemyHealth.UMG_EnemyHealth_C" null self))
  (`WidgetComponent.SetWidget` (`self.HealthBar`) _returnvalue))

(event `self.PawnSensing.OnSeePawn`
  (params (Pawn :type "Pawn Object Reference"))
  ;[1 1 1] 看到的玩家传递给行为树的attacktarget
  (bind _asbp_first_person_character (cast `/Game/FirstPerson/Blueprints/BP_FirstPersonCharacter` Pawn))
  (`BlackboardComponent.SetValueAsObject` (`AIBlueprintHelperLibrary.GetBlackboard` null) "AttackTarget" _asbp_first_person_character))

(event `PlayAttackEnemy`
  (bind _returnvalue (`self.K2_GetActorLocation`))
  (bind _notifyname (`|PlayMontage` (`self.Mesh`) (`KismetArrayLibrary.Array_Random` (`self.AttackMontageList`)))
    (:`OnCompleted`
      ;[1 1 1] 分发者告诉全世界：动画播完了
      (`self.ED_AttackEnd` :!label _label))
    (:`OnInterrupted`
      (goto _label))
    (:`OnNotifyBegin`
      ;[1 1 1] 当攻击动画播放到蒙太奇通知的时候，会触发
      (switch `name` _notifyname
        (:`EnemyAttackDamage`
          ;[1 1 1] 在敌人前方两米进行球体检测碰到的物体
          (bind _outhits (`KismetSystemLibrary.SphereTraceMultiForObjects` _returnvalue (+ _returnvalue (* (`self.GetActorForwardVector`) 200.0)) 50.0 (`|MakeArray` "ObjectTypeQuery3" :!type "EObjectTypeQuery Enum")))
          (for _array_element _outhits
            (bind _asbp_first_person_character (cast `/Game/FirstPerson/Blueprints/BP_FirstPersonCharacter` (`.HitActor` (`GameplayStatics.BreakHitResult` _array_element))))
            (`/Game/FirstPerson/Blueprints/BP_FirstPersonCharacter.GetDamage` _asbp_first_person_character (`KismetMathLibrary.RandomFloatInRange` 20.0 30.0))
            (break)))))))

(event `AttackDamage`
  (params (DamageValue :type "Float (double-precision)"))
  ;[1 1 1] 敌人受到伤害减血，如果不小于0播放伤害动画并停止移动；如果为0设置死亡，播放死亡动画
  (if (> (`self.Health`) 0.0)
    (bind _output_get (set `self.Health` (- (`self.Health`) DamageValue)))
    (if (<= _output_get 0.0)
      (set `self.isDeath` true)
      ;[1 1 1] 敌人死亡，停止逻辑树
      (`BrainComponent.StopLogic` (`AIController.BrainComponent` (`self.AIController`)) "")
      (`PrimitiveComponent.SetCollisionEnabled` (`self.CapsuleComponent`) "NoCollision")
      (`PrimitiveComponent.SetCollisionEnabled` (`self.Mesh`) "NoCollision")
      (`ActorComponent.K2_DestroyComponent` (`self.HealthBar`))
      (bind _asbp_first_person_game_mode (cast `/Game/FirstPerson/Blueprints/BP_FirstPersonGameMode` (`GameplayStatics.GetGameMode`)))
      (`/Game/FirstPerson/Blueprints/BP_FirstPersonGameMode.SetEnemyDeath` _asbp_first_person_game_mode self)
      (else
        ;[1 1 1] 敌人血量不为0，敌人受到攻击时，将攻击目标设置为玩家
        (`BlackboardComponent.SetValueAsObject` (`AIBlueprintHelperLibrary.GetBlackboard` null) "AttackTarget" (`GameplayStatics.GetPlayerCharacter` 0))
        (`|PlayMontage` (`self.Mesh`) (`self.HitMontage`)
          (:`then`
            (`CharacterMovementComponent.SetMovementMode` (`self.CharacterMovement`) "MOVE_None" 0)
            (set `CharacterMovementComponent.MaxWalkSpeed` 0.0 (`self.CharacterMovement`)))
          (:`OnCompleted`
            (`CharacterMovementComponent.SetMovementMode` (`self.CharacterMovement`) "MOVE_Walking" 0)
            (set `CharacterMovementComponent.MaxWalkSpeed` 375.0 (`self.CharacterMovement`))))))))

(fn `UserConstructionScript`)